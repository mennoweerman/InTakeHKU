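; BP_MinableBase is a base Blueprint for minable objects that yield item drops when mined.
; MineItem drops a random number of single ItemName units, scaled by MaxDropAmount, through the player's InventorySystem ServerDropItem, then calls MCUpdate.
; GetDropLocation traces toward a point below a random forward-cone offset from the player and returns the hit location, though MineItem does not call it.
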(fn `GetDropLocation`
  (params (PlayerRef :type "/Game/ThirdPerson/Blueprints/BP_ThirdPersonCharacter Object Reference"))
  (returns (Location :type "Vector Structure"))
  (bind _returnvalue (`self.K2_GetActorLocation` PlayerRef))
  (`/Engine/EditorBlueprintResources/StandardMacros.IsValid` PlayerRef
    (:`Is Valid`
      (bind _outhit (`KismetSystemLibrary.LineTraceSingle` _returnvalue (- (+ _returnvalue (* (`KismetMathLibrary.RandomUnitVectorInConeInDegrees` (`self.GetActorForwardVector` PlayerRef) 45.0) (`self.DropDistance`))) (0.0 0.0 500.0)) "TraceTypeQuery1"))
      (return (`.Location` (`GameplayStatics.BreakHitResult` _outhit))))))

(fn `MineItem`
  (params (PlayerRef :type "/Game/ThirdPerson/Blueprints/BP_ThirdPersonCharacter Object Reference"))
  (returns (`DidMine?` :type Boolean))
  (bind _inventorysystem (`/Game/ThirdPerson/Blueprints/BP_ThirdPersonCharacter.InventorySystem` PlayerRef))
  (for _ (range (+ (+ (`KismetMathLibrary.RandomInteger` (`self.MaxDropAmount`)) 1) 1))
    (`/Game/Blueprints/InventorySystem/InventorySystem.Server_DropItem` _inventorysystem (`self.ItemName`) 1))
  (`/Game/Blueprints/InventorySystem/InventorySystem.MC_Update` _inventorysystem)
  (return true))

(fn `UserConstructionScript`)