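; BP_ItemBase is a pickup item, apparently a base class, that grants experience to the player when touched.
; It caches the BP_GameHandler actor on BeginPlay and fires PickedUpItem when the player character overlaps its PickUpSphere.
; PickedUpItem adds the item's ExperienceToGain to the handler's Experience, triggers its level-up check, then destroys the item.
; The CheckForStackPossibile function is an empty stub.
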(event `self.ReceiveBeginPlay`
  (bind _returnvalue (`GameplayStatics.GetActorOfClass` "/Game/Blueprints/BP_GameHandler.BP_GameHandler_C"))
  (set `self.GameHandlerRef` _returnvalue))

(event `self.PickUpSphere.OnComponentBeginOverlap`
  (params (OverlappedComponent :type "PrimitiveComponent Object Reference") (OtherActor :type "Actor Object Reference") (OtherComp :type "PrimitiveComponent Object Reference") (OtherBodyIndex :type Integer) (bFromSweep :type Boolean) (SweepResult :type "HitResult Structure (by ref)"))
  (if (== OtherActor (`GameplayStatics.GetPlayerCharacter` 0))
    (`/Game/Blueprints/I_ItemPickedUp.PickedUpItem` self)))

(event `/Game/Blueprints/I_ItemPickedUp.PickedUpItem`
  (params (PickedUpItem :type "/Game/Blueprints/BP_ItemBase Object Reference"))
  (bind _gamehandlerref (`self.GameHandlerRef`))
  (set `/Game/Blueprints/BP_GameHandler.Experience` (+ (`/Game/Blueprints/BP_GameHandler.Experience` _gamehandlerref) (`/Game/Blueprints/BP_ItemBase.ExperienceToGain` PickedUpItem)) _gamehandlerref)
  (`/Game/Blueprints/BP_GameHandler.CheckIfLevelUp` (`self.GameHandlerRef`))
  (`self.K2_DestroyActor`))

(fn `CheckForStackPossibile`)

(fn `UserConstructionScript`)