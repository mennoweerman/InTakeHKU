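; Actor component that turns its owner into a pickup item for the inventory system, carrying an item ID row and a quantity.
; On BeginPlay it enables replication on the owner.
; Its interact event adds the item to the player character's InventorySystem and destroys the owner only when the add succeeds.
; A LookAt function returns an empty string.
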(event `self.ReceiveBeginPlay`
  (`Actor.SetReplicates` (`self.GetOwner`) true))

(event `/Game/Blueprints/InventorySystem/I_InteractInterface.InteractWith`
  (params (PlayerCharacter :type "/Game/ThirdPerson/Blueprints/BP_ThirdPersonCharacter Object Reference"))
  (bind _inventorysystem (`/Game/ThirdPerson/Blueprints/BP_ThirdPersonCharacter.InventorySystem` PlayerCharacter))
  (bind (_itemid_datatable _itemid_rowname) (break `DataTableRowHandle` (`self.ItemID`)))
  (`/Engine/EditorBlueprintResources/StandardMacros.IsValid` _inventorysystem
    (:`Is Valid`
      (bind _succes_ (`/Game/Blueprints/InventorySystem/InventorySystem.AddToInventory` _inventorysystem _itemid_rowname (`self.Quantity`)))
      (if _succes_
        (`Actor.K2_DestroyActor` (`self.GetOwner`))))))

(fn `LookAt`
  (returns (Message :type Text))
  (return ""))