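; Base pickup item actor for the inventory system that spins in place and supplies a "Pick up" prompt when looked at.
; Tick advances the actor's yaw by TurnSpeed scaled by delta time.
; LookAt resolves the ItemDataComponent's ItemID data table row and formats the prompt from the item's Name.
; The pickup action itself is not handled in this graph.
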(event `self.ReceiveTick`
  (params (DeltaSeconds :type "Float (single-precision)"))
  (bind (_returnvalue_roll _returnvalue_pitch _returnvalue_yaw) (`KismetMathLibrary.BreakRotator` (`self.K2_GetActorRotation`)))
  (`self.K2_SetActorRotation` (`KismetMathLibrary.MakeRotator` 0.0 0.0 (+ _returnvalue_yaw (* DeltaSeconds (`self.TurnSpeed`))))))

(fn `LookAt`
  (returns (Message :type Text))
  (bind (_itemid_datatable _itemid_rowname) (break `DataTableRowHandle` (`/Game/Blueprints/InventorySystem/ItemDataComponent.ItemID` (`self.ItemDataComponent`))))
  (bind _returnvalue (`|GetDataTableRow` _itemid_datatable _itemid_rowname)
    (:`then`
      (return (`|FormatText` "Pick up {Item}" (`.Name_2_0316D6EB4D103B72EB98CAAB1E0E77EC` (break `/Game/Blueprints/InventorySystem/Structs/Item/S_ItemStruct` _returnvalue)))))))

(fn `UserConstructionScript`)